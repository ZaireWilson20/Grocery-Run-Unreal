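; MainHUD creates the player's crosshair widget and toggles its focus indicator when the first-person character hovers over something.
; On BeginPlay it casts player 0 to BP_FirstPersonCharacter, binds to its hover enter and exit events, and adds the Crosshair widget to the viewport with focus hidden.
; The hover handlers call EnteredHover and ExitedHover, which show or hide that focus through CrosshairFocus, so updates are event-driven without Tick.
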(event Custom|HandleHoverEnter
  (CallFunction|EnteredHover))

(event Custom|HandleHoverExit
  (CallFunction|ExitedHover))

(event EventBeginPlay
  (bind _asbp_first_person_character (Utilities|Casting|CastToBP_FirstPersonCharacter (Game|GetPlayerCharacter 0)))
  (bind _output_get (Variables|Default|SetPlayerCharacter _asbp_first_person_character))
  (EventDispatchers|BindEventtoOnHoverEnter _output_get (delegate Custom|HandleHoverEnter))
  (bind _returnvalue (UserInterface|CreateWidget "/Game/FirstPerson/UI/Crosshair.Crosshair_C"))
  (bind _output_get_2 (Variables|Default|SetCrosshairWidget _returnvalue))
  (UserInterface|Viewport|AddtoViewport _output_get_2 0)
  (EventDispatchers|BindEventtoOnHoverExit _output_get (delegate Custom|HandleHoverExit))
  (Default|CrosshairFocus _output_get_2 "Hidden"))

(event Collision|EventActorBeginOverlap
  (params (OtherActor :type Actor%20Object%20Reference)))

(event EventTick
  (params (DeltaSeconds :type Float%20%28single-precision%29)))

(fn ConstructionScript)

(fn EnteredHover
  (bind _crosshairwidget (Variables|Default|GetCrosshairWidget))
  ;[1 1 1] Enable Crosshair
  (if (!= _crosshairwidget 0)
    (Default|CrosshairFocus _crosshairwidget "Visible")))

(fn ExitedHover
  (bind _crosshairwidget (Variables|Default|GetCrosshairWidget))
  ;[1 1 1] Disable Crosshair
  (if (!= _crosshairwidget 0)
    (Default|CrosshairFocus _crosshairwidget "Hidden")))